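; PhysicsTruck is a physics-driven vehicle prop that loops from its spawn point, changing between four vehicle meshes.
; On BeginPlay it records the spawn location and picks a random mesh through a randomly seeded stream.
; Each tick it applies a constant world rotation (despite the ConstantForce name) and checks height.
; Below LowestZ it teleports back, cuts velocity to a tenth and rerolls the mesh.
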(event `self.ReceiveBeginPlay`
  (`self.Begin`))

(event `self.ReceiveActorBeginOverlap`
  (params (OtherActor :type "Actor Object Reference")))

(event `self.ReceiveTick`
  (params (DeltaSeconds :type "Float (single-precision)"))
  (`self.ConstantForce` DeltaSeconds)
  (`self.Check Teleport`))

(fn `Begin`
  (set `self.SpawnPoint` (`SceneComponent.K2_GetComponentLocation` (`self.Truck`)))
  (`self.RandomTruck`))

(fn `Check Teleport`
  (bind _truck (`self.Truck`))
  (if (< (.z (`SceneComponent.K2_GetComponentLocation` (`self.Truck`))) (`self.Lowest Z`))
    (`SceneComponent.K2_SetWorldLocation` (`self.Truck`) (`self.SpawnPoint`) false)
    (`PrimitiveComponent.SetPhysicsLinearVelocity` _truck (/ (`SceneComponent.GetComponentVelocity` _truck) 10.0) false "None")
    (`self.RandomTruck`)))

(fn `ConstantForce`
  (params (DeltaTime :type "Float (double-precision)"))
  (`SceneComponent.K2_AddWorldRotation` (`self.Truck`) (* (`self.ConstantRotator`) DeltaTime) false))

(fn `RandomTruck`
  (bind _truck (`self.Truck`))
  (bind _truck_2 (`self.Truck`))
  (switch `/Game/Bigger/Data/TruckType` (cast `/Game/Bigger/Data/TruckType` (`KismetMathLibrary.Conv_IntToByte` (`KismetMathLibrary.RandomIntegerInRangeFromStream` 0 3 (`KismetMathLibrary.MakeRandomStream` (`KismetMathLibrary.RandomInteger` 17)))))
    (:`NewEnumerator0`
      (`StaticMeshComponent.SetStaticMesh` _truck_2 "/Game/Bigger/Models/pickup_truck.pickup_truck"))
    (:`NewEnumerator1`
      (`StaticMeshComponent.SetStaticMesh` _truck_2 "/Game/Bigger/Models/school_bus.school_bus"))
    (:`NewEnumerator2`
      (`StaticMeshComponent.SetStaticMesh` _truck "/Game/Bigger/Models/sports_car.sports_car"))
    (:`NewEnumerator3`
      (`StaticMeshComponent.SetStaticMesh` _truck "/Game/Bigger/Models/ice_cream_truck.ice_cream_truck"))))

(fn `UserConstructionScript`)