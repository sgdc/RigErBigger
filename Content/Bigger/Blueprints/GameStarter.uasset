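; GameStarter sets up a local split-screen truck race when play begins.
; It reads player count and game mode from the "local" save, creates the extra players and gathers their pawns into a shared array.
; Each BiggerCharacter receives its ID, that array, the mode, an ID-based truck, lap target and spawn setup.
; HandleScreens then adds full, half or quarter HUDs to suit the player count, followed by a shared TimerHUD.
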(event `self.ReceiveBeginPlay`
  (bind _asbigger_character (cast `/Game/Bigger/Blueprints/BiggerCharacter` (`GameplayStatics.GetPlayerPawn` 0)))
  (`KismetArrayLibrary.Array_Add` (`self.PlayerArray`) _asbigger_character)
  (bind _returnvalue (`GameplayStatics.LoadGameFromSlot` "local"))
  (bind _asmy_game_save (cast `/Game/Bigger/Data/MyGameSave` _returnvalue))
  (bind _returnvalue_2 (- (`/Game/Bigger/Data/MyGameSave.NumberOfPlayers` _asmy_game_save) 1))
  (for _index (range 1 (+ _returnvalue_2 1))
    (`GameplayStatics.CreatePlayer` _index)
    (bind _asbigger_character_2 (cast `/Game/Bigger/Blueprints/BiggerCharacter` (`GameplayStatics.GetPlayerPawn` _index)))
    (`KismetArrayLibrary.Array_Add` (`self.PlayerArray`) _asbigger_character_2))
  (for _index_2 (range (+ _returnvalue_2 1))
    (bind _asbigger_character_3 (cast `/Game/Bigger/Blueprints/BiggerCharacter` (`GameplayStatics.GetPlayerPawn` _index_2)))
    (set `/Game/Bigger/Blueprints/BiggerCharacter.PlayerID` _index_2 _asbigger_character_3)
    (set `/Game/Bigger/Blueprints/BiggerCharacter.PlayerArray` (`self.PlayerArray`) _asbigger_character_3)
    (set `/Game/Bigger/Blueprints/BiggerCharacter.Game Mode` (`/Game/Bigger/Data/MyGameSave.Game Mode` _asmy_game_save) _asbigger_character_3)
    (`/Game/Bigger/Blueprints/BiggerCharacter.Change Truck` _asbigger_character_3 (cast `/Game/Bigger/Data/TruckType` (`KismetMathLibrary.Conv_IntToByte` _index_2)))
    (set `/Game/Bigger/Blueprints/BiggerCharacter.UseY` (`self.UseY`) _asbigger_character_3)
    (`/Game/Bigger/Blueprints/BiggerCharacter.Set Spawn` _asbigger_character_3)
    (set `/Game/Bigger/Blueprints/BiggerCharacter.Total Laps Needed` (`self.totalLapsNeeded`) _asbigger_character_3))
  (`self.HandleScreens` _returnvalue_2)
  (bind _returnvalue_3 (`|CreateWidget` "/Game/Bigger/HUD/TimerHUD.TimerHUD_C"))
  (set `/Game/Bigger/HUD/TimerHUD.isSinglePlayer` (== _returnvalue_2 0) _returnvalue_3)
  (`UserWidget.AddToViewport` _returnvalue_3 0))

(fn `HandleScreens`
  (params (Selection :type Integer))
  (bind _item (`KismetArrayLibrary.Array_Get` (`self.PlayerArray`)))
  (bind _item_2 (`KismetArrayLibrary.Array_Get` (`self.PlayerArray`)))
  (switch `int` Selection
    (:`Default`
      (return))
    (:`0`
      (bind _returnvalue (`Controller.CastToPlayerController` (`Pawn.GetController` _item)))
      (bind _returnvalue_2 (`|CreateWidget` "/Game/Bigger/HUD/RedneckHUD.RedneckHUD_C" _returnvalue))
      (set `/Game/Bigger/HUD/RedneckHUD.ID` (`/Game/Bigger/Blueprints/BiggerCharacter.PlayerID` _item) _returnvalue_2)
      (`/Game/Bigger/HUD/RedneckHUD.MyConstruct` _returnvalue_2)
      (`UserWidget.AddToPlayerScreen` _returnvalue_2 0))
    (:`1`
      (for _array_element (`self.PlayerArray`)
        (bind _returnvalue_3 (`Controller.CastToPlayerController` (`Pawn.GetController` _array_element)))
        (bind _returnvalue_4 (`|CreateWidget` "/Game/Bigger/HUD/RedneckHalfHUD.RedneckHalfHUD_C" _returnvalue_3))
        (set `/Game/Bigger/HUD/RedneckHalfHUD.ID` (`/Game/Bigger/Blueprints/BiggerCharacter.PlayerID` _array_element) _returnvalue_4)
        (`/Game/Bigger/HUD/RedneckHalfHUD.MyConstruct` _returnvalue_4)
        (`UserWidget.AddToPlayerScreen` _returnvalue_4 0)))
    (:`2`
      (bind _returnvalue_5 (`Controller.CastToPlayerController` (`Pawn.GetController` _item_2)))
      (bind _returnvalue_6 (`|CreateWidget` "/Game/Bigger/HUD/RedneckHalfHUD.RedneckHalfHUD_C" _returnvalue_5))
      (set `/Game/Bigger/HUD/RedneckHalfHUD.ID` (`/Game/Bigger/Blueprints/BiggerCharacter.PlayerID` _item_2) _returnvalue_6)
      (`/Game/Bigger/HUD/RedneckHalfHUD.MyConstruct` _returnvalue_6)
      (`UserWidget.AddToPlayerScreen` _returnvalue_6 0)
      (for _index (range 1 3)
        (bind _item_3 (`KismetArrayLibrary.Array_Get` (`self.PlayerArray`) _index))
        (bind _returnvalue_7 (`Controller.CastToPlayerController` (`Pawn.GetController` _item_3)))
        (bind _returnvalue_8 (`|CreateWidget` "/Game/Bigger/HUD/RedneckQuartileHUD.RedneckQuartileHUD_C" _returnvalue_7))
        (set `/Game/Bigger/HUD/RedneckQuartileHUD.ID` (`/Game/Bigger/Blueprints/BiggerCharacter.PlayerID` _item_3) _returnvalue_8)
        (`/Game/Bigger/HUD/RedneckQuartileHUD.MyConstruct` _returnvalue_8)
        (`UserWidget.AddToPlayerScreen` _returnvalue_8 0)))
    (:`3`
      (for _array_element_2 (`self.PlayerArray`)
        (bind _returnvalue_9 (`Controller.CastToPlayerController` (`Pawn.GetController` _array_element_2)))
        (bind _returnvalue_10 (`|CreateWidget` "/Game/Bigger/HUD/RedneckQuartileHUD.RedneckQuartileHUD_C" _returnvalue_9))
        (set `/Game/Bigger/HUD/RedneckQuartileHUD.ID` (`/Game/Bigger/Blueprints/BiggerCharacter.PlayerID` _array_element_2) _returnvalue_10)
        (`/Game/Bigger/HUD/RedneckQuartileHUD.MyConstruct` _returnvalue_10)
        (`UserWidget.AddToPlayerScreen` _returnvalue_10 0)))))

(fn `UserConstructionScript`)