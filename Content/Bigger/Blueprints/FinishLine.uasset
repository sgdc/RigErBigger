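; Finish line trigger for a multiplayer lap race that counts laps and declares the winner.
; At BeginPlay it passes the required lap total to every GameStarter.
; Overlapping BiggerCharacters that reached the highest checkpoint get a player-count-scaled sound, a new respawn point, a checkpoint reset and another lap.
; The first to complete all laps is sent to TimerHUD widgets as winner; otherwise that player's Checkpoint indicator materials reset.
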(event `self.ReceiveBeginPlay`
  (bind _outactors (`GameplayStatics.GetAllActorsOfClass` "/Game/Bigger/Blueprints/GameStarter.GameStarter_C"))
  (for _array_element _outactors
    (set `/Game/Bigger/Blueprints/GameStarter.totalLapsNeeded` (`self.Total Needed Number Of Laps`) _array_element)))

(event `self.Box.OnComponentBeginOverlap`
  (params (OtherActor :type "Actor Object Reference") (OtherComp :type "PrimitiveComponent Object Reference") (OtherBodyIndex :type Integer) (bFromSweep :type Boolean) (SweepResult :type "HitResult Structure (by ref)"))
  (bind _asbigger_character (cast `/Game/Bigger/Blueprints/BiggerCharacter` OtherActor))
  (bind _currentcheckpointid (`/Game/Bigger/Blueprints/BiggerCharacter.CurrentCheckpointID` _asbigger_character))
  (if (== _currentcheckpointid (`self.Highest Checkpoint ID`))
    (`GameplayStatics.PlaySoundAtLocation` "/Game/Bigger/Sounds/RB_Finish_Line.RB_Finish_Line" (`SceneComponent.K2_GetComponentLocation` (`self.Box`)) (/ 1.0 (* (`KismetArrayLibrary.Array_Length` (`/Game/Bigger/Blueprints/BiggerCharacter.PlayerArray` _asbigger_character)) (`/Game/Bigger/Blueprints/BiggerCharacter.VolumeDivisor` _asbigger_character))) 1.0 0.0 "/Game/Bigger/Data/RocketAttenuation.RocketAttenuation")
    (`|ExecutionSequence`
      (:`then_0`
        (set `/Game/Bigger/Blueprints/BiggerCharacter.respawnPoint` (`self.GetTransform` _asbigger_character) _asbigger_character :!label _label))
      (:`then_1`
        (set `/Game/Bigger/Blueprints/BiggerCharacter.CurrentCheckpointID` -1 _asbigger_character)
        (bind _output_get (set `/Game/Bigger/Blueprints/BiggerCharacter.Laps Completed` (+ (`/Game/Bigger/Blueprints/BiggerCharacter.Laps Completed` _asbigger_character) 1) _asbigger_character))
        (if (and (== _output_get (`self.Total Needed Number Of Laps`)) (not (`self.RaceFinished`)))
          (set `self.RaceFinished` true)
          (bind _foundwidgets (`WidgetBlueprintLibrary.GetAllWidgetsOfClass` "/Game/Bigger/HUD/TimerHUD.TimerHUD_C"))
          (for _array_element _foundwidgets
            (bind _astimer_hud (cast `/Game/Bigger/HUD/TimerHUD` _array_element))
            (set `/Game/Bigger/HUD/TimerHUD.Winner ID` (`/Game/Bigger/Blueprints/BiggerCharacter.PlayerID` _asbigger_character) _astimer_hud)
            (set `/Game/Bigger/HUD/TimerHUD.Mode` "NewEnumerator2" _astimer_hud))
          (else
            (bind _outactors (`GameplayStatics.GetAllActorsOfClass` "/Game/Bigger/Blueprints/Checkpoint.Checkpoint_C"))
            (for _array_element_2 _outactors
              (if (== (`/Game/Bigger/Blueprints/Checkpoint.ID` _array_element_2) 0)
                (bind _item (`KismetArrayLibrary.Array_Get` (`/Game/Bigger/Blueprints/Checkpoint.IndicatorArray` _array_element_2) (+ (`/Game/Bigger/Blueprints/BiggerCharacter.PlayerID` _asbigger_character) 1)))
                (`PrimitiveComponent.SetMaterial` _item 0 "/Game/Bigger/Models/MyMaterials/GoalRed.GoalRed")
                (else
                  (`PrimitiveComponent.SetMaterial` _item 0 "/Game/Bigger/Models/MyMaterials/DarkGrey.DarkGrey"))))))))
    (elif (== _currentcheckpointid -1)
      (goto _label))))

(fn `UserConstructionScript`)