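; Main menu controller that creates the racing game's menu screens and routes menu input between them.
; Begin creates the widgets, most holding a reference back to it, and shows the title screen.
; CurrentHUD acts as the state: inputs are forwarded to that screen, and ChangeHUDs swaps the visible widget.
; With a missing or IsStarting settings save, it applies settings, forces 1080p fullscreen and saves a fresh object with the flag cleared.
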(event `InputAction|Menu Left`
  (:`Pressed`
    (switch `/Game/Bigger/Data/MainMenuEnums/CurrentHUD` (`self.CurrentHUD`)
      (:`NewEnumerator1`
        (`/Game/Bigger/HUD/MainMenu/2ModeSelect.ArrowReceived` (`self.ModeSelectHUD`)))
      (:`NewEnumerator2`
        (`/Game/Bigger/HUD/MainMenu/3NumberOfRacers.Change Player Num` (`self.NumRacersHUD`) -1))
      (:`NewEnumerator3`
        (`/Game/Bigger/HUD/MainMenu/4RaceMapSelect.Left Received` (`self.RaceMapHUD`)))
      (:`NewEnumerator5`
        (`/Game/Bigger/HUD/MainMenu/6Settings.Left Received` (`self.SettingsHUD`))))))

(event `InputAction|Menu Back`
  (:`Pressed`
    (`GameplayStatics.PlaySound2D` "/Game/Bigger/Sounds/RBMenuBack.RBMenuBack")
    (switch `/Game/Bigger/Data/MainMenuEnums/CurrentHUD` (`self.CurrentHUD`)
      (:`NewEnumerator0`
        (`/Game/Bigger/HUD/MainMenu/1TitleHUD.ChangeSelectedButton` (`self.TitleHUD`) "NewEnumerator2"))
      (:`NewEnumerator1`
        (`self.ChangeHUDs` "NewEnumerator0" :!label _label))
      (:`NewEnumerator2`
        (goto _label))
      (:`NewEnumerator3`
        (`self.ChangeHUDs` "NewEnumerator2" :!label _label_2))
      (:`NewEnumerator4`
        (goto _label_2))
      (:`NewEnumerator5`
        (goto _label))
      (:`NewEnumerator6`
        (goto _label)))))

(event `InputAction|Menu Up`
  (:`Pressed`
    (switch `/Game/Bigger/Data/MainMenuEnums/CurrentHUD` (`self.CurrentHUD`)
      (:`NewEnumerator0`
        (`/Game/Bigger/HUD/MainMenu/1TitleHUD.Up Received` (`self.TitleHUD`)))
      (:`NewEnumerator5`
        (`/Game/Bigger/HUD/MainMenu/6Settings.Up Received` (`self.SettingsHUD`))))))

(event `InputAction|Menu Down`
  (:`Pressed`
    (switch `/Game/Bigger/Data/MainMenuEnums/CurrentHUD` (`self.CurrentHUD`)
      (:`NewEnumerator0`
        (`/Game/Bigger/HUD/MainMenu/1TitleHUD.Down Received` (`self.TitleHUD`)))
      (:`NewEnumerator5`
        (`/Game/Bigger/HUD/MainMenu/6Settings.Down Received` (`self.SettingsHUD`))))))

(event `InputAction|Menu Right`
  (:`Pressed`
    (switch `/Game/Bigger/Data/MainMenuEnums/CurrentHUD` (`self.CurrentHUD`)
      (:`NewEnumerator1`
        (`/Game/Bigger/HUD/MainMenu/2ModeSelect.ArrowReceived` (`self.ModeSelectHUD`)))
      (:`NewEnumerator2`
        (`/Game/Bigger/HUD/MainMenu/3NumberOfRacers.Change Player Num` (`self.NumRacersHUD`) 1))
      (:`NewEnumerator3`
        (`/Game/Bigger/HUD/MainMenu/4RaceMapSelect.Right Received` (`self.RaceMapHUD`)))
      (:`NewEnumerator5`
        (`/Game/Bigger/HUD/MainMenu/6Settings.Right Received` (`self.SettingsHUD`))))))

(event `InputAction|Menu Enter`
  (:`Pressed`
    (`GameplayStatics.PlaySound2D` "/Game/Bigger/Sounds/RBMenuSelect.RBMenuSelect")
    (switch `/Game/Bigger/Data/MainMenuEnums/CurrentHUD` (`self.CurrentHUD`)
      (:`NewEnumerator0`
        (`/Game/Bigger/HUD/MainMenu/1TitleHUD.Enter Received` (`self.TitleHUD`)))
      (:`NewEnumerator1`
        (`/Game/Bigger/HUD/MainMenu/2ModeSelect.Enter Received` (`self.ModeSelectHUD`)))
      (:`NewEnumerator2`
        (`/Game/Bigger/HUD/MainMenu/3NumberOfRacers.Enter Received` (`self.NumRacersHUD`)))
      (:`NewEnumerator3`
        (`/Game/Bigger/HUD/MainMenu/4RaceMapSelect.Enter Received` (`self.RaceMapHUD`)))
      (:`NewEnumerator4`
        (`/Game/Bigger/HUD/MainMenu/5BattleMapSelect.Enter Received` (`self.BattleMapHUD`)))
      (:`NewEnumerator5`
        (`/Game/Bigger/HUD/MainMenu/6Settings.Enter Received` (`self.SettingsHUD`)))
      (:`NewEnumerator6`
        (`self.ChangeHUDs` "NewEnumerator0")))))

(event `self.ReceiveBeginPlay`
  (`self.Begin`))

(fn `Begin`
  (`|ExecutionSequence`
    (:`then_0`
      (bind _returnvalue (`|CreateWidget` "/Game/Bigger/HUD/MainMenu/1TitleHUD.1TitleHUD_C"))
      (bind _output_get (set `self.TitleHUD` _returnvalue))
      (set `/Game/Bigger/HUD/MainMenu/1TitleHUD.Owner` self _output_get)
      (bind _returnvalue_2 (`|CreateWidget` "/Game/Bigger/HUD/MainMenu/2ModeSelect.2ModeSelect_C"))
      (bind _output_get_2 (set `self.ModeSelectHUD` _returnvalue_2))
      (set `/Game/Bigger/HUD/MainMenu/2ModeSelect.Owner` self _output_get_2)
      (bind _returnvalue_3 (`|CreateWidget` "/Game/Bigger/HUD/MainMenu/3NumberOfRacers.3NumberOfRacers_C"))
      (bind _output_get_3 (set `self.NumRacersHUD` _returnvalue_3))
      (set `/Game/Bigger/HUD/MainMenu/3NumberOfRacers.Owner` self _output_get_3)
      (bind _returnvalue_4 (`|CreateWidget` "/Game/Bigger/HUD/MainMenu/4RaceMapSelect.4RaceMapSelect_C"))
      (bind _output_get_4 (set `self.RaceMapHUD` _returnvalue_4))
      (set `/Game/Bigger/HUD/MainMenu/4RaceMapSelect.Owner` self _output_get_4)
      (bind _returnvalue_5 (`|CreateWidget` "/Game/Bigger/HUD/MainMenu/5BattleMapSelect.5BattleMapSelect_C"))
      (bind _output_get_5 (set `self.BattleMapHUD` _returnvalue_5))
      (set `/Game/Bigger/HUD/MainMenu/5BattleMapSelect.Owner` self _output_get_5)
      (bind _returnvalue_6 (`|CreateWidget` "/Game/Bigger/HUD/MainMenu/7Controls.7Controls_C"))
      (set `self.ControlsHUD` _returnvalue_6)
      (bind _returnvalue_7 (`|CreateWidget` "/Game/Bigger/HUD/MainMenu/6Settings.6Settings_C"))
      (bind _output_get_6 (set `self.SettingsHUD` _returnvalue_7))
      (set `/Game/Bigger/HUD/MainMenu/6Settings.Owner` self _output_get_6)
      (bind _returnvalue_8 (`GameplayStatics.LoadGameFromSlot` "settings"))
      (bind _assettings_save (cast `/Game/Bigger/Data/SettingsSave` _returnvalue_8)
        (:`then`
          (if (`/Game/Bigger/Data/SettingsSave.isStarting` _assettings_save)
            (`/Game/Bigger/HUD/MainMenu/6Settings.Apply Settings` _output_get_6 :!label _label)
            (`KismetSystemLibrary.ExecuteConsoleCommand` "r.SetRes 1920x1080f")
            (bind _returnvalue_9 (`GameplayStatics.CreateSaveGameObject` "/Game/Bigger/Data/SettingsSave.SettingsSave_C"))
            (bind _assettings_save_2 (cast `/Game/Bigger/Data/SettingsSave` _returnvalue_9))
            (set `/Game/Bigger/Data/SettingsSave.isStarting` false _assettings_save_2)
            (`GameplayStatics.SaveGameToSlot` _assettings_save_2 "settings")))
        (:`CastFailed`
          (goto _label))))
    (:`then_1`
      (`self.ChangeHUDs` "NewEnumerator0"))))

(fn `ChangeHUDs`
  (params (`To Change To` :type "/Game/Bigger/Data/MainMenuEnums/CurrentHUD Enum"))
  (bind _output_get (set `self.CurrentHUD` `To Change To`))
  (`|ExecutionSequence`
    (:`then_0`
      (`Widget.RemoveFromParent` (`self.TitleHUD`))
      (`Widget.RemoveFromParent` (`self.ModeSelectHUD`))
      (`Widget.RemoveFromParent` (`self.NumRacersHUD`))
      (`Widget.RemoveFromParent` (`self.RaceMapHUD`))
      (`Widget.RemoveFromParent` (`self.BattleMapHUD`))
      (`Widget.RemoveFromParent` (`self.SettingsHUD`))
      (`Widget.RemoveFromParent` (`self.ControlsHUD`)))
    (:`then_1`
      (switch `/Game/Bigger/Data/MainMenuEnums/CurrentHUD` _output_get
        (:`NewEnumerator0`
          (`UserWidget.AddToViewport` (`self.TitleHUD`) 0))
        (:`NewEnumerator1`
          (`UserWidget.AddToViewport` (`self.ModeSelectHUD`) 0))
        (:`NewEnumerator2`
          (`UserWidget.AddToViewport` (`self.NumRacersHUD`) 0))
        (:`NewEnumerator3`
          (`UserWidget.AddToViewport` (`self.RaceMapHUD`) 0))
        (:`NewEnumerator4`
          (`UserWidget.AddToViewport` (`self.BattleMapHUD`) 0))
        (:`NewEnumerator5`
          (`UserWidget.AddToViewport` (`self.SettingsHUD`) 0))
        (:`NewEnumerator6`
          (`UserWidget.AddToViewport` (`self.ControlsHUD`) 0))))))

(fn `UserConstructionScript`)