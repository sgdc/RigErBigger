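; Rocket projectile fired by a truck (BiggerCharacter) that flies straight along its local X axis, spawning trail explosion emitters each tick.
; While CanCollide is set, box overlaps ignore checkpoints, finish lines, itself, its owner and zero-health trucks.
; Other trucks receive GetHit, and they or any other overlap detonate it.
; An expired timer destroys it silently; impact volume scales down with player count.
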(event `FireSound`
  (bind _owningtruck (`self.OwningTruck`))
  (`GameplayStatics.PlaySoundAttached` "/Game/Bigger/Sounds/MissleLaunch.MissleLaunch" (`self.Rocket`) "None" (`KismetMathLibrary.Conv_DoubleToVector` (/ 1.0 (* (`KismetArrayLibrary.Array_Length` (`/Game/Bigger/Blueprints/BiggerCharacter.PlayerArray` _owningtruck)) (`/Game/Bigger/Blueprints/BiggerCharacter.VolumeDivisor` _owningtruck)))) "KeepRelativeOffset" false 0.25 0.9 0.0 "/Game/Bigger/Data/RocketLaunchAttenuation.RocketLaunchAttenuation"))

(event `self.ReceiveTick`
  (params (DeltaSeconds :type "Float (single-precision)"))
  (`self.Move` DeltaSeconds)
  (`self.TimedDeath` DeltaSeconds))

(event `self.BoxCollision.OnComponentBeginOverlap`
  (params (OtherActor :type "Actor Object Reference") (OtherComp :type "PrimitiveComponent Object Reference") (OtherBodyIndex :type Integer) (bFromSweep :type Boolean) (SweepResult :type "HitResult Structure (by ref)"))
  (if (`self.CanCollide`)
    (cast `/Game/Bigger/Blueprints/Checkpoint` OtherActor
      (:`CastFailed`
        (cast `/Game/Bigger/Blueprints/FinishLine` OtherActor
          (:`CastFailed`
            (bind _asrocket (cast `/Game/Bigger/Blueprints/Rocket` OtherActor)
              (:`then`
                (if (!= _asrocket self)
                  (bind _asbigger_character (cast `/Game/Bigger/Blueprints/BiggerCharacter` OtherActor :!label _label)
                    (:`then`
                      (if (`KismetSystemLibrary.IsValid` (`self.OwningTruck`))
                        (if (!= _asbigger_character (`self.OwningTruck`))
                          (if (not (== (`/Game/Bigger/Blueprints/BiggerCharacter.Health` _asbigger_character) 0))
                            (`/Game/Bigger/Blueprints/BiggerCharacter.GetHit` _asbigger_character self)
                            (`self.Death` false :!label _label_2)))))
                    (:`CastFailed`
                      (goto _label_2)))))
              (:`CastFailed`
                (goto _label)))))))))

(fn `Death`
  (params (Fizzle :type Boolean))
  (bind _owningtruck (`self.OwningTruck`))
  (if (not Fizzle)
    (`GameplayStatics.SpawnEmitterAtLocation` "/Game/StarterContent/Particles/P_Explosion.P_Explosion" (`self.K2_GetActorLocation`))
    (`GameplayStatics.PlaySoundAtLocation` "/Game/Bigger/Sounds/impact.impact" (`self.K2_GetActorLocation`) (/ 1.0 (* (`KismetArrayLibrary.Array_Length` (`/Game/Bigger/Blueprints/BiggerCharacter.PlayerArray` _owningtruck)) (`/Game/Bigger/Blueprints/BiggerCharacter.VolumeDivisor` _owningtruck))) 1.0 0.0 "/Game/Bigger/Data/RocketAttenuation.RocketAttenuation"))
  (`self.K2_DestroyActor`)
  (return))

(fn `Move`
  (params (DeltaTime :type "Float (double-precision)"))
  (bind _sphere (`self.Sphere`))
  (`self.K2_AddActorLocalOffset` (`KismetMathLibrary.MakeVector` (* (`self.RocketSpeed`) DeltaTime)))
  (`/Engine/EditorBlueprintResources/StandardMacros.IsValid` _sphere
    (:`Is Valid`
      (`GameplayStatics.SpawnEmitterAtLocation` "/Game/StarterContent/Particles/P_Explosion2.P_Explosion2" (`SceneComponent.K2_GetComponentLocation` _sphere)))))

(fn `TimedDeath`
  (params (DeltaTime :type "Float (double-precision)"))
  (bind _output_get (set `self.TimeLimit` (- (`self.TimeLimit`) DeltaTime)))
  (if (<= _output_get 0.0)
    (`self.Death` true)))

(fn `UserConstructionScript`)