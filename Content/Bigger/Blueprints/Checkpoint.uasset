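; Checkpoint actor that tracks each player's progress through an ID-ordered sequence and updates their respawn point.
; Box overlap advances a BiggerCharacter only if its checkpoint ID is one lower, then plays a sound scaled down by player count and volume divisor.
; Four indicators, indexed by player ID, turn green here and goal-red on the next checkpoint, found by searching all Checkpoint actors; checkpoint zero starts goal-red.
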(event `self.ReceiveBeginPlay`
  (bind _indicatorarray (`self.IndicatorArray`))
  (`KismetArrayLibrary.Array_Add` _indicatorarray (`self.Indicator1`))
  (`KismetArrayLibrary.Array_Add` _indicatorarray (`self.Indicator2`))
  (`KismetArrayLibrary.Array_Add` _indicatorarray (`self.Indicator3`))
  (`KismetArrayLibrary.Array_Add` _indicatorarray (`self.Indicator4`))
  (if (== (`self.ID`) 0)
    (for _array_element (`self.IndicatorArray`)
      (`PrimitiveComponent.SetMaterial` _array_element 0 "/Game/Bigger/Models/MyMaterials/GoalRed.GoalRed"))))

(event `self.Box.OnComponentBeginOverlap`
  (params (OtherActor :type "Actor Object Reference") (OtherComp :type "PrimitiveComponent Object Reference") (OtherBodyIndex :type Integer) (bFromSweep :type Boolean) (SweepResult :type "HitResult Structure (by ref)"))
  (bind _asbigger_character (cast `/Game/Bigger/Blueprints/BiggerCharacter` OtherActor))
  (if (== (`/Game/Bigger/Blueprints/BiggerCharacter.CurrentCheckpointID` _asbigger_character) (- (`self.ID`) 1))
    (set `/Game/Bigger/Blueprints/BiggerCharacter.respawnPoint` (`self.GetTransform` _asbigger_character) _asbigger_character)
    (`GameplayStatics.PlaySoundAtLocation` "/Game/Bigger/Sounds/RB_checkpoint_sound.RB_checkpoint_sound" (`SceneComponent.K2_GetComponentLocation` (`self.Box`)) (/ 1.0 (* (`KismetArrayLibrary.Array_Length` (`/Game/Bigger/Blueprints/BiggerCharacter.PlayerArray` _asbigger_character)) (`/Game/Bigger/Blueprints/BiggerCharacter.VolumeDivisor` _asbigger_character))) 1.0 0.0 "/Game/Bigger/Data/RocketAttenuation.RocketAttenuation")
    (set `/Game/Bigger/Blueprints/BiggerCharacter.CurrentCheckpointID` (`self.ID`) _asbigger_character)
    (`PrimitiveComponent.SetMaterial` (`KismetArrayLibrary.Array_Get` (`self.IndicatorArray`) (+ (`/Game/Bigger/Blueprints/BiggerCharacter.PlayerID` _asbigger_character) 1)) 0 "/Game/Bigger/Models/MyMaterials/Green.Green")
    (`PrimitiveComponent.SetMaterial` (`self.CorrectIndicator`) 0 "/Game/Bigger/Models/MyMaterials/Green.Green")
    (bind _outactors (`GameplayStatics.GetAllActorsOfClass` "Checkpoint_C"))
    (for _array_element _outactors
      (if (== (`/Game/Bigger/Blueprints/Checkpoint.ID` _array_element) (+ (`self.ID`) 1))
        (`PrimitiveComponent.SetMaterial` (`KismetArrayLibrary.Array_Get` (`/Game/Bigger/Blueprints/Checkpoint.IndicatorArray` _array_element) (+ (`/Game/Bigger/Blueprints/BiggerCharacter.PlayerID` _asbigger_character) 1)) 0 "/Game/Bigger/Models/MyMaterials/GoalRed.GoalRed")
        (`PrimitiveComponent.SetMaterial` (`self.CorrectIndicator`) 0 "/Game/Bigger/Models/MyMaterials/RocketRed.RocketRed")))))

(fn `UserConstructionScript`)