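; Boost pad actor that boosts a BiggerCharacter when it overlaps the pad.
; On overlap it calls the character's Boost with the pad's world rotation as direction, plus its magnitude, static-boost and force-jump settings.
; The pad then shows a boosting material, and a retriggerable delay restores the normal one, so repeated hits extend the highlight.
; The construction script applies the normal material initially.
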(event `self.ReceiveBeginPlay`)

(event `self.ReceiveActorBeginOverlap`
  (params (OtherActor :type "Actor Object Reference"))
  (bind _asbigger_character (cast `/Game/Bigger/Blueprints/BiggerCharacter` OtherActor))
  (`/Game/Bigger/Blueprints/BiggerCharacter.Boost` _asbigger_character (`SceneComponent.K2_GetComponentRotation` (`self.Pad`)) (`self.Boost Multiply Magnitude`) (`self.Static Boost`) (`self.forceJump`))
  (`PrimitiveComponent.SetMaterial` (`self.Pad`) 0 (`self.BoostingMaterial`))
  (`KismetSystemLibrary.RetriggerableDelay` 0.75)
  (`PrimitiveComponent.SetMaterial` (`self.Pad`) 0 (`self.NormalMaterial`)))

(event `self.ReceiveTick`
  (params (DeltaSeconds :type "Float (single-precision)")))

(fn `UserConstructionScript`
  (`PrimitiveComponent.SetMaterial` (`self.Pad`) 0 (`self.NormalMaterial`)))