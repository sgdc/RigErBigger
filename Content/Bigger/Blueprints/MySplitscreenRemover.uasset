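; A helper actor that clears in-game HUD widgets from the screen, apparently for tearing down splitscreen play.
; KillAllNonTitleHUDs finds all top-level RedneckHUD, RedneckHalfHUD, RedneckQuartileHUD and TimerHUD widgets and removes each from its parent.
; The event graph and construction script are empty, so the function runs only when called from outside.
; Despite the asset name, it only removes widgets and does not touch players or viewports.
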(event `self.ReceiveBeginPlay`)

(event `self.ReceiveActorBeginOverlap`
  (params (OtherActor :type "Actor Object Reference")))

(event `self.ReceiveTick`
  (params (DeltaSeconds :type "Float (single-precision)")))

(fn `KillAllNonTitleHUDs`
  (bind _foundwidgets (`WidgetBlueprintLibrary.GetAllWidgetsOfClass` "/Game/Bigger/HUD/RedneckHUD.RedneckHUD_C"))
  (for _array_element _foundwidgets
    (`Widget.RemoveFromParent` _array_element))
  (bind _foundwidgets_2 (`WidgetBlueprintLibrary.GetAllWidgetsOfClass` "/Game/Bigger/HUD/RedneckHalfHUD.RedneckHalfHUD_C"))
  (for _array_element_2 _foundwidgets_2
    (`Widget.RemoveFromParent` _array_element_2))
  (bind _foundwidgets_3 (`WidgetBlueprintLibrary.GetAllWidgetsOfClass` "/Game/Bigger/HUD/RedneckQuartileHUD.RedneckQuartileHUD_C"))
  (for _array_element_3 _foundwidgets_3
    (`Widget.RemoveFromParent` _array_element_3))
  (bind _foundwidgets_4 (`WidgetBlueprintLibrary.GetAllWidgetsOfClass` "/Game/Bigger/HUD/TimerHUD.TimerHUD_C"))
  (for _array_element_4 _foundwidgets_4
    (`Widget.RemoveFromParent` _array_element_4)))

(fn `UserConstructionScript`)